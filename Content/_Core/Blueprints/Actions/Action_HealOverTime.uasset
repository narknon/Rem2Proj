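; Action_HealOverTime is an action Blueprint that outlines a heal-over-time effect, with start and tick-style events.
; It declares functions for percent-of-max-health healing, modifiers, scalars, healing owner, per-second rate, eligibility and regen.
; All of these are empty or return defaults, so no healing logic or wiring is present.
; Only the inspect-info and debug-text overrides do anything, passing through to the parent.
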(event `self.OnActionStart`)

(event `OnHOT`)

(fn `CanDoHealing`
  (returns (Out :type Boolean))
  (return false))

(fn `DetermineHealthRegen`)

(fn `DoHealing`)

(fn `Get Calculated Healing Per Second`
  (returns (ReturnValue :type "Float (double-precision)"))
  (return 0.0))

(fn `GetDebugText`
  (returns (ReturnValue :type String))
  (bind _returnvalue (`parent.GetDebugText`))
  (return _returnvalue))

(fn `GetHealingMod`
  (returns (HealingMod :type "Float (double-precision)"))
  (return 0.0))

(fn `GetHealingOwner`
  (returns (Owner :type "Actor Object Reference"))
  (return null))

(fn `GetHealingScalar`
  (returns (Out :type "Float (double-precision)"))
  (return 0.0))

(fn `GetHealingToApply`
  (returns (ReturnValue :type "Float (double-precision)"))
  (return 0.0))

(fn `GetPercentOfMaxHealthToHeal`
  (returns (HealthPercent :type "Float (double-precision)"))
  (return 0.0))

(fn `GetUnmodifiedHealPercentage`
  (returns (ReturnValue :type "Float (double-precision)"))
  (return 0.0))

(fn `ModifyInspectInfo`
  (params (Actor :type "Actor Object Reference") (InspectLevel :type Integer) (Info :type "InspectInfo Structure (by ref)"))
  (returns (Rtn :type Boolean))
  (bind _rtn (`parent.ModifyInspectInfo` Actor InspectLevel Info))
  (return _rtn))