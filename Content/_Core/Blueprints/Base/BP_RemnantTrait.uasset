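; BP_RemnantTrait is a base Blueprint for traits, providing shared helpers and overridable hooks.
; GetCharacter casts the owner to CharacterGunfire, and IsTargetAggro reports whether a target pawn's Gunfire AI controller has a valid current target.
; GetFunctionalDescription returns the Description, and ModifyInspectInfo defers to the parent.
; The preview-info and action functions are empty stubs, with DoAction returning zero.
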(fn `DoAction`
  (params (ActionBP :type "ActionBase Class Reference (by ref)"))
  (returns (ActionID :type Integer))
  (return 0))

(fn `DoActionOnTarget`
  (params (Action :type "ActionBase Class Reference") (Target :type "Actor Object Reference")))

(fn `GetCharacter`
  (returns (Out :type "CharacterGunfire Object Reference"))
  (bind _ascharacter_gunfire (cast `CharacterGunfire` (`self.GetOwner`)))
  (return _ascharacter_gunfire))

(fn `GetFunctionalDescription`
  (params (Actor :type "Actor Object Reference") (Level :type Integer) (ReadOnlyInfo :type "InspectInfo Structure"))
  (returns (InfoText :type Text))
  (return (`self.Description`)))

(fn `IsTargetAggro`
  (params (Target :type "Actor Object Reference"))
  (returns (Out :type Boolean))
  (bind _aspawn (cast `Pawn` Target)
    (:`then`
      (bind _asaicontroller_gunfire (cast `AIControllerGunfire` (`Pawn.GetController` _aspawn))
        (:`then`
          (`/Engine/EditorBlueprintResources/StandardMacros.IsValid` (`AIControllerGunfire.GetCurrentTarget` _asaicontroller_gunfire)
            (:`Is Valid`
              (return true))
            (:`Is Not Valid`
              _)))
        (:`CastFailed`
          _)))
    (:`CastFailed`
      _))
  (return false))

(fn `ModifyInspectInfo`
  (params (Actor :type "Actor Object Reference") (InspectLevel :type Integer) (Info :type "InspectInfo Structure (by ref)"))
  (returns (Rtn :type Boolean))
  (bind _rtn (`parent.ModifyInspectInfo` Actor InspectLevel Info))
  (return _rtn))

(fn `ModifyPreviewInfo`
  (params (InspectInfo :type "InspectInfo Structure (by ref)")))